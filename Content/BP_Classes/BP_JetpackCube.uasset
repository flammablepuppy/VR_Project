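; BP_JetpackCube is a held VR pickup that works as a jetpack, pushing the owning vrPlayer along the cube's up direction.
; Trigger pulls above a small dead zone apply thrust scaled by ThrustPower and the analog trigger value.
; A falling player gets the thrust added directly to movement velocity, while a player who is not falling is lifted with an additive LaunchCharacter call.
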(event `self.BPTriggerPull`
  (params (Value :type "Float (single-precision)"))
  (bind _asvr_player (cast `vrPlayer` (`ActorComponent.GetOwner` (`self.GetOwningMC`)) :!pure true))
  (bind _returnvalue (* (`KismetMathLibrary.GetUpVector` (`SceneComponent.K2_GetComponentRotation` (`self.PickupMesh`))) (* (`self.ThrustPower`) Value)))
  (bind _returnvalue_2 (`Pawn.GetMovementComponent` _asvr_player))
  (if (> Value 0.1)
    (if (`NavMovementComponent.IsFalling` _returnvalue_2)
      (set `MovementComponent.Velocity` (+ (`MovementComponent.Velocity` _returnvalue_2) _returnvalue) _returnvalue_2)
      (else
        (`Character.LaunchCharacter` _asvr_player _returnvalue false false)))))

(fn `UserConstructionScript`)