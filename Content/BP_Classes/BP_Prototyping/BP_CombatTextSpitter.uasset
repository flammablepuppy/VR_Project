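; Prototyping actor that continuously spits test floating damage numbers from its static mesh's location.
; From BeginPlay, DisplayText casts the first player controller's pawn to BP_vrDebugPawn and calls its SpawnDamageFloat with a random damage value.
; DisplayText then calls itself after a short Delay, forming an endless repeating loop.
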(event `self.ReceiveBeginPlay`
  (`self.DisplayText`))

(event `DisplayText`
  (`/Game/BP_Classes/vrPawn/BP_vrDebugPawn.SpawnDamageFloat` (cast `/Game/BP_Classes/vrPawn/BP_vrDebugPawn` (`Controller.K2_GetPawn` (`GameplayStatics.GetPlayerController` 0)) :!pure true) (`SceneComponent.K2_GetComponentLocation` (`self.StaticMesh`)) (`KismetMathLibrary.RandomFloatInRange` 1.0 999.0))
  (`KismetSystemLibrary.Delay` 0.2)
  (`self.DisplayText`))

(fn `UserConstructionScript`)