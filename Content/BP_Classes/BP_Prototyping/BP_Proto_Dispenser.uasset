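; BP_Proto_Dispenser is a prototype dispenser that spawns BP_RollingMine actors in bursts and destroys itself on death.
; An actor overlap on Trigger with a full counter, or a vrPlayer entering TriggerVolume, starts a recursive, delayed SpawnCycle.
; Each mine gets a velocity-change impulse along the dispenser mesh's negative up axis, then CallSpawnMines runs with its HealthStats.
; After a burst, non-SingleShooter dispensers refill following a cooldown and optionally loop.
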(event `self.ReceiveBeginPlay`
  (set `self.SpawnCounter` (`self.SpawnsPerCycle`))
  (add `HealthStats.OnDeath` (`self.HealthStats`) (delegate `Destroy`)))

(event `Destroy`
  (params (DyingActor :type "Actor Object Reference"))
  (`self.K2_DestroyActor`))

(event `self.Trigger.OnActorBeginOverlap`
  (params (OverlappedActor :type "Actor Object Reference") (OtherActor :type "Actor Object Reference"))
  (if (not (< (`self.SpawnCounter`) (`self.SpawnsPerCycle`)))
    (`self.SpawnCycle`)))

(event `SpawnCycle`
  (bind _spawncounter (`self.SpawnCounter`))
  (if (> _spawncounter 0)
    (`/Engine/EditorBlueprintResources/StandardMacros.DecrementInt` _spawncounter
      (:`  `
        (bind _returnvalue (`|SpawnActorFromClass` "/Game/BP_Classes/BP_RollingMine.BP_RollingMine_C" (`KismetMathLibrary.MakeTransform` (`SceneComponent.K2_GetComponentLocation` (`self.SpawnSphere`))) "AdjustIfPossibleButAlwaysSpawn" "OverrideRootScale" null null))
        (bind _returnvalue_2 (`RollingMine.GetMesh` _returnvalue))
        (`PrimitiveComponent.AddImpulse` _returnvalue_2 (* (`SceneComponent.GetUpVector` (`self.DispenserMesh`)) -2300.0) "None" true)
        (bind _returnvalue_3 (`RollingMine.GetHealthStats` _returnvalue))
        (`self.SpawnMines` _returnvalue_3)
        (`KismetSystemLibrary.Delay` (`self.SpawnDelay`))
        (`self.SpawnCycle`)))
    (elif (not (`self.bSingleShooter`))
      (`KismetSystemLibrary.Delay` (`self.CycleDelay`))
      (set `self.SpawnCounter` (`self.SpawnsPerCycle`))
      (if (`self.bLoopsSpawning`)
        (`self.SpawnCycle`)))))

(event `self.TriggerVolume.OnComponentBeginOverlap`
  (params (OverlappedComponent :type "PrimitiveComponent Object Reference") (OtherActor :type "Actor Object Reference") (OtherComp :type "PrimitiveComponent Object Reference") (OtherBodyIndex :type Integer) (bFromSweep :type Boolean) (SweepResult :type "HitResult Structure (by ref)"))
  (cast `vrPlayer` OtherActor)
  (`self.SpawnCycle`))

(fn `UserConstructionScript`)