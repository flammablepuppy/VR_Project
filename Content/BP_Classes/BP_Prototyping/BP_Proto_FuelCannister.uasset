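; A prototype fuel cannister pickup that spins at a random speed and refuels the VR player's handheld thrusters.
; On sphere overlap it gathers HandThrusters from the player's left and right hands, refuelling only when the right hand holds one.
; FuelToGive is split evenly between them as a percentage, then the cannister signals collection, plays a pickup sound and destroys itself.
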(event `self.ReceiveBeginPlay`
  ;[1 1 1] Spin these things
  (`self.K2_SetActorRotation` (`KismetMathLibrary.MakeRotator` 0.0 (`KismetMathLibrary.RandomFloatInRange` 8.0 30.0)))
  (set `RotatingMovementComponent.RotationRate` (`KismetMathLibrary.MakeRotator` 0.0 0.0 (`KismetMathLibrary.RandomFloatInRange` 90.0 270.0)) (`self.RotatingMovement`)))

(event `self.OverlapSphere.OnComponentBeginOverlap`
  (params (OverlappedComponent :type "PrimitiveComponent Object Reference") (OtherActor :type "Actor Object Reference") (OtherComp :type "PrimitiveComponent Object Reference") (OtherBodyIndex :type Integer) (bFromSweep :type Boolean) (SweepResult :type "HitResult Structure (by ref)"))
  ;[1 1 1] When overlapped, save references to and hand thrusters that overlapping player is holding.
  (bind _asvr_player (cast `vrPlayer` (`ActorComponent.GetOwner` OtherComp)))
  (bind _leftheldobject (`vrPlayer.LeftHeldObject` _asvr_player))
  (`/Engine/EditorBlueprintResources/StandardMacros.IsValid` _leftheldobject
    (:`Is Valid`
      (bind _ashand_thruster (cast `HandThruster` _leftheldobject))
      (`KismetArrayLibrary.Array_AddUnique` (`self.ThrustersToFuel`) _ashand_thruster))
    (:`Is Not Valid`
      _))
  (bind _rightheldobject (`vrPlayer.RightHeldObject` _asvr_player))
  (`/Engine/EditorBlueprintResources/StandardMacros.IsValid` _rightheldobject
    (:`Is Valid`
      (bind _ashand_thruster_2 (cast `HandThruster` _rightheldobject))
      (`KismetArrayLibrary.Array_AddUnique` (`self.ThrustersToFuel`) _ashand_thruster_2)
      (`self.Refuel`)
      (`self.OnCannisterCollected`))))

(event `Refuel`
  (bind _thrusterstofuel (`self.ThrustersToFuel`))
  ;[1 1 1] Add fuel to all thrusters saved in the array.
  (for _array_element _thrusterstofuel
    (`HandThruster.AddFuel` _array_element (/ (`self.FuelToGive`) (`KismetMathLibrary.Conv_IntToDouble` (`KismetArrayLibrary.Array_Length` _thrusterstofuel))) true))
  (`GameplayStatics.SpawnSoundAtLocation` "/Game/BP_Classes/BP_Prototyping/ThrusterFuel/FuelPickup_cue.FuelPickup_cue" (`self.K2_GetActorLocation`) (struct) 1.0 1.0 0.0 null null)
  (`self.K2_DestroyActor`))

(fn `UserConstructionScript`)