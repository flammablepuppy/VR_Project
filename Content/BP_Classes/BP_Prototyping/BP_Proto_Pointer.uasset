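; Prototype pointer that rotates an arrow mesh to track the current race checkpoint.
; Each Tick it gets the checkpoint from RaceGameMode and aligns the arrow's X axis with the normalized vector from that checkpoint to its owner.
; A validity check that would show or hide the arrow is left unconnected, so Tick rotates it without any check.
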(event `self.ReceiveTick`
  (params (DeltaSeconds :type "Float (single-precision)"))
  (`SceneComponent.K2_SetWorldRotation` (`self.ArrowMesh`) (`KismetMathLibrary.Conv_VectorToRotator` (`KismetMathLibrary.Normal` (- (`self.K2_GetActorLocation` (`self.GetOwner`)) (`self.K2_GetActorLocation` (`RaceGameMode.GetCurrentCheckpoint` (cast `RaceGameMode` (`GameplayStatics.GetGameMode`) :!pure true)))))) false false))

(fn `UserConstructionScript`)