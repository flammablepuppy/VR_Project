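; Checkpoint actor that saves its location to the VR player's health component when first touched.
; A timeline animates the mesh's height and yaw, and activation swaps its material and plays a sound.
; It binds to the player's death event to optionally spawn a list of actors above itself.
; One-time checkpoints also bind to respawn, which zeroes the saved location and destroys the checkpoint.
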(event `self.ReceiveBeginPlay`
  (bind _checkpointmesh (`self.CheckpointMesh`))
  (bind (_direction _mesh_z_curve _rotation) (`Timeline|MeshZ` :!via `PlayFromStart`)
    (:`Update`
      (`SceneComponent.K2_SetRelativeLocation` _checkpointmesh (`KismetMathLibrary.MakeVector` 0.0 0.0 _mesh_z_curve) false false)
      (`SceneComponent.K2_SetRelativeRotation` _checkpointmesh (`KismetMathLibrary.MakeRotator` 0.0 0.0 _rotation) false false))))

(event `self.CheckpointMesh.OnComponentBeginOverlap`
  (params (OverlappedComponent :type "PrimitiveComponent Object Reference") (OtherActor :type "Actor Object Reference") (OtherComp :type "PrimitiveComponent Object Reference") (OtherBodyIndex :type Integer) (bFromSweep :type Boolean) (SweepResult :type "HitResult Structure (by ref)"))
  (if (not (`self.bCheckpointUsed`))
    (bind _asvr_player (cast `vrPlayer` OtherActor))
    (set `self.bCheckpointUsed` true)
    (bind _healthstatscomp (`vrPlayer.HealthStatsComp` _asvr_player))
    (set `HealthStats.CheckpointLocation` (`SceneComponent.K2_GetComponentLocation` (`self.CheckpointRoot`)) _healthstatscomp)
    (`PrimitiveComponent.SetMaterial` (`self.CheckpointMesh`) 0 "/Game/BP_Classes/SigPistol/StaticMeshes_Materials/GreenSights.GreenSights")
    (add `HealthStats.OnDeath` _healthstatscomp (delegate `OnDeathBoundEvent`))
    (`GameplayStatics.PlaySoundAtLocation` "/Game/BP_Classes/BP_Prototyping/Checkpoint/Checkpoint_Cue.Checkpoint_Cue" (`SceneComponent.K2_GetComponentLocation` (`self.CheckpointMesh`)) (struct) 1.0 1.0 0.0 null null null)
    (if (`self.bOneTimeUse`)
      (add `HealthStats.OnRespawn` _healthstatscomp (delegate `OnRespawnBoundEvent`)))))

(event `OnDeathBoundEvent`
  (bind (_returnvalue_location _returnvalue_rotation) (`KismetMathLibrary.BreakTransform` (`SceneComponent.K2_GetComponentToWorld` (`self.CheckpointMesh`))))
  (if (`self.bSpawnsItems`)
    (for _array_element (`self.ActorsToSpawn`)
      (`|SpawnActorFromClass` _array_element (`KismetMathLibrary.MakeTransform` (+ (`KismetMathLibrary.MakeVector` 0.0 0.0 100.0) _returnvalue_location) _returnvalue_rotation) "AlwaysSpawn" "OverrideRootScale" null null))))

(event `OnRespawnBoundEvent`
  (set `HealthStats.CheckpointLocation` (0.0 0.0 0.0) (`vrPlayer.HealthStatsComp` (stale `self.CheckpointMesh.OnComponentBeginOverlap` _asvr_player)))
  (`self.K2_DestroyActor`))

(fn `UserConstructionScript`)