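; BP_HealthShot is a single-use VR health injector that heals a player when its trigger is pulled.
; Pulling past halfway spends the charge and turns a mesh material red, even if no player is in range.
; It then takes the first VrPlayer overlapping the needle scan volume and, if their health is below maximum, heals them by applying negative damage.
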(event `self.BPTriggerPull`
  (params (Value :type "Float (single-precision)"))
  (bind _overlappingactors (`PrimitiveComponent.GetOverlappingActors` (`self.NeedleScanVolume`) "/Script/VR_Project.vrPlayer"))
  (bind _output (`|GetArrayItem` _overlappingactors))
  (bind _healthstatscomp (`vrPlayer.HealthStatsComp` (cast `vrPlayer` _output :!pure true)))
  (if (> Value 0.5)
    (if (`self.bHasCharge`)
      (set `self.bHasCharge` false)
      (`PrimitiveComponent.SetMaterial` (`self.PickupMesh`) 2 "/Game/BP_Classes/BP_Prototyping/HealthShot/m_healthshot_red.m_healthshot_red")
      (if (> (`KismetArrayLibrary.Array_Length` _overlappingactors) 0)
        (if (< (`HealthStats.CurrentHealth` _healthstatscomp) (`HealthStats.MaximumHealth` _healthstatscomp))
          (`GameplayStatics.ApplyDamage` _output -75.0 null null "/Script/Engine.DamageType"))))))

(fn `UserConstructionScript`)