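; Prototype VR holster that snaps a held pickup into place when it is released inside the holster bounds.
; Overlap stores one hand-held vrPickup as the target, and ending the overlap clears it.
; Tick polls for a missing owning motion controller, then drops and snaps the target to the bounds, or re-enables pickup if the holster already owns it.
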(event `self.HolsterBounds.OnComponentBeginOverlap`
  (params (OverlappedComponent :type "PrimitiveComponent Object Reference") (OtherActor :type "Actor Object Reference") (OtherComp :type "PrimitiveComponent Object Reference") (OtherBodyIndex :type Integer) (bFromSweep :type Boolean) (SweepResult :type "HitResult Structure (by ref)"))
  (if (not (`KismetSystemLibrary.IsValid` (`self.HolsterTarget`)))
    (bind _asstatic_mesh_component (cast `StaticMeshComponent` OtherComp))
    (bind _asvr_pickup (cast `vrPickup` (`ActorComponent.GetOwner` _asstatic_mesh_component)))
    (if (`KismetSystemLibrary.IsValid` (`vrPickup.GetOwningMC` _asvr_pickup))
      (set `self.HolsterTarget` _asvr_pickup))))

(event `self.ReceiveTick`
  (params (DeltaSeconds :type "Float (single-precision)"))
  (bind _holstertarget (`self.HolsterTarget`))
  (if (`KismetSystemLibrary.IsValid` (`vrPickup.GetOwningMC` _holstertarget))
    _
    (elif (== (`self.GetOwner` _holstertarget) self)
      (`vrPickup.SetPickupEnabled` _holstertarget true)
      (else
        (`vrPickup.Drop` _holstertarget)
        (`vrPickup.SnapInitiate` _holstertarget (`self.HolsterBounds`) "None")
        (`KismetSystemLibrary.Delay` 0.5)))))

(event `self.HolsterBounds.OnComponentEndOverlap`
  (params (OverlappedComponent :type "PrimitiveComponent Object Reference") (OtherActor :type "Actor Object Reference") (OtherComp :type "PrimitiveComponent Object Reference") (OtherBodyIndex :type Integer))
  (if (== (`ActorComponent.GetOwner` OtherComp) (`self.HolsterTarget`))
    (set `self.HolsterTarget` null)))

(fn `UserConstructionScript`)