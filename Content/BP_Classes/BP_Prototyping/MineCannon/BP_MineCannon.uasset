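; BP_MineCannon is a cannon that starts firing floating mines once its PawnSensing component first sees a pawn.
; Each shot spawns a BP_FloatingMine at the CannonBase Muzzle socket and launches it forward with a velocity-change impulse.
; Mine tracking stays off briefly after launch, then switches on.
; FireMine re-calls itself after a delay, so firing repeats with no stop condition.
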(event `self.PawnSensing.OnSeePawn`
  (params (Pawn :type "Pawn Object Reference"))
  (if (not (`self.bActivatedMySensing`))
    (set `self.bActivatedMySensing` true)
    (`self.FireMine`)))

(event `FireMine`
  (bind _cannonbase (`self.CannonBase`))
  (bind (_returnvalue_location _returnvalue_rotation) (`KismetMathLibrary.BreakTransform` (`SceneComponent.GetSocketTransform` _cannonbase "Muzzle" "RTS_World")))
  (bind _returnvalue (`|SpawnActorFromClass` "/Game/BP_Classes/FloatingMine/BP_FloatingMine.BP_FloatingMine_C" (`SceneComponent.GetSocketTransform` _cannonbase "Muzzle" "RTS_World") "AdjustIfPossibleButAlwaysSpawn" "OverrideRootScale" null null))
  (`FloatingMine.SetTrackingOn` _returnvalue false)
  (`PrimitiveComponent.AddImpulse` (`FloatingMine.MineMesh` _returnvalue) (* (`KismetMathLibrary.GetForwardVector` _returnvalue_rotation) 1000.0) "None" true)
  (`KismetSystemLibrary.Delay` 0.5)
  (`FloatingMine.SetTrackingOn` _returnvalue true)
  (`KismetSystemLibrary.Delay` 2.5)
  (`self.FireMine`))

(fn `UserConstructionScript`)