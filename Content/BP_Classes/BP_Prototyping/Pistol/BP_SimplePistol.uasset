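; BP_SimplePistol is a VR pistol pickup that fires bullets when the motion controller trigger is pulled past a threshold.
; Each shot uses a round, then a short delay gates the next.
; Bullets spawn at the Muzzle socket, pushed forward in proportion to the controller owner's speed, with that owner set as theirs.
; BeginPlay fills the magazine and links the ammo counter widget to the pistol.
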(event `self.ReceiveBeginPlay`
  (set `/Game/BP_Classes/BP_Prototyping/Pistol/UI_PistolAmmo.OwningPistol` self (cast `/Game/BP_Classes/BP_Prototyping/Pistol/UI_PistolAmmo` (`WidgetComponent.GetUserWidgetObject` (`self.AmmoCounter`)) :!pure true))
  (set `self.RoundsRemaining` (`self.MaxRounds`)))

(event `self.BPTriggerPull`
  (params (Value :type "Float (single-precision)"))
  (bind _pickupmesh (`self.PickupMesh`))
  (bind (_returnvalue_location _returnvalue_rotation _returnvalue_scale) (`KismetMathLibrary.BreakTransform` (`SceneComponent.GetSocketTransform` _pickupmesh "Muzzle" "RTS_World")))
  (bind _returnvalue (`ActorComponent.GetOwner` (`self.GetOwningMC`)))
  (if (> Value 0.3)
    (if (`self.bReadyToFire`)
      (if (> (`self.RoundsRemaining`) 0.0)
        (set `self.bReadyToFire` false)
        (set `self.RoundsRemaining` (- (`self.RoundsRemaining`) 1.0))
        (`|SpawnActorFromClass` "/Game/BP_Classes/BP_Prototyping/Pistol/BP_Bullet.BP_Bullet_C" (`KismetMathLibrary.MakeTransform` (+ _returnvalue_location (* (`SceneComponent.GetForwardVector` _pickupmesh) (* (`KismetMathLibrary.VSize` (`self.GetVelocity` _returnvalue)) 0.02))) _returnvalue_rotation _returnvalue_scale) "AdjustIfPossibleButAlwaysSpawn" "OverrideRootScale" _returnvalue null)
        (`KismetSystemLibrary.Delay` 0.2)
        (set `self.bReadyToFire` true)))))

(fn `UserConstructionScript`)