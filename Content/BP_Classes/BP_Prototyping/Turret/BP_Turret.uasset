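; Prototype turret that targets a VR player within its detection sphere, fires bullets and is destroyed through its health component.
; Sphere overlap starts scanning; Tick picks the nearest player only while none is held, saving their location once.
; Yaw and barrel pitch interpolate toward that location while bullets spawn from the muzzle socket on a short cooldown.
; The line trace records distance but always marks line of sight true.
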(event `self.HealthStats.OnDeath`
  (`KismetSystemLibrary.PrintString` "KILLED TURRET")
  (`self.K2_DestroyActor`))

(event `Fire`
  (bind (_returnvalue_location _returnvalue_rotation) (`KismetMathLibrary.BreakTransform` (`SceneComponent.GetSocketTransform` (`self.Barrel`) "Muzzle" "RTS_World")))
  (`|SpawnActorFromClass` "/Game/BP_Classes/BP_Prototyping/Pistol/BP_Bullet.BP_Bullet_C" (`KismetMathLibrary.MakeTransform` _returnvalue_location _returnvalue_rotation) "AdjustIfPossibleButAlwaysSpawn" "OverrideRootScale" null null)
  (set `self.bOffCooldown` false)
  (`KismetSystemLibrary.Delay` 0.2)
  (set `self.bOffCooldown` true))

(event `UpdatePitch`
  (bind _barrelpitchpivot (`self.BarrelPitchPivot`))
  (bind (_returnvalue_roll _returnvalue_pitch _returnvalue_yaw) (`KismetMathLibrary.BreakRotator` (`SceneComponent.K2_GetComponentRotation` (`self.Turret`))))
  (bind (_returnvalue_roll_2 _returnvalue_pitch_2) (`KismetMathLibrary.BreakRotator` (`KismetMathLibrary.FindLookAtRotation` (`SceneComponent.K2_GetComponentLocation` _barrelpitchpivot) (`self.TargetLocation`))))
  (`SceneComponent.K2_SetWorldRotation` (`self.BarrelPitchPivot`) (`KismetMathLibrary.RInterpTo` (`SceneComponent.K2_GetComponentRotation` _barrelpitchpivot) (`KismetMathLibrary.MakeRotator` 0.0 _returnvalue_pitch_2 _returnvalue_yaw) (`self.DeltaTime`) (`self.PitchRate`)) false false))

(event `UpdateAzimuth`
  (bind _turret (`self.Turret`))
  (bind (_returnvalue_roll _returnvalue_pitch _returnvalue_yaw) (`KismetMathLibrary.BreakRotator` (`KismetMathLibrary.FindLookAtRotation` (`SceneComponent.K2_GetComponentLocation` _turret) (`self.TargetLocation`))))
  (`SceneComponent.K2_SetWorldRotation` (`self.Turret`) (`KismetMathLibrary.RInterpTo` (`SceneComponent.K2_GetComponentRotation` _turret) (`KismetMathLibrary.MakeRotator` 0.0 0.0 _returnvalue_yaw) (`self.DeltaTime`) (`self.AzimuthRate`)) false false))

(event `self.ReceiveTick`
  (params (DeltaSeconds :type "Float (single-precision)"))
  (set `self.DeltaTime` DeltaSeconds)
  (if (`self.bScanOn`)
    (if (not (`KismetSystemLibrary.IsValid` (`self.ClosestPlayer`)))
      (`self.GetClostestPlayer`))
    (if (`self.bTargetInLOS`)
      (`self.UpdateAzimuth`)
      (`self.UpdatePitch`)
      (if (`self.bOffCooldown`)
        (`self.Fire`)))))

(event `CheckClosestestPlayerLOS`
  (bind _outhit (`KismetSystemLibrary.LineTraceSingle` (`SceneComponent.GetSocketLocation` (`self.Barrel`) "Muzzle") (`SceneComponent.K2_GetComponentLocation` (`Character.CapsuleComponent` (`self.ClosestPlayer`))) "TraceTypeQuery1"))
  (set `self.bTargetInLOS` true)
  (bind _output_get (set `self.DistanceToTarget` (`.Distance` (`GameplayStatics.BreakHitResult` _outhit))))
  (set `self.TargetLocation` (`SceneComponent.K2_GetComponentLocation` (`Character.CapsuleComponent` (`self.ClosestPlayer`)))))

(event `self.Sphere.OnComponentBeginOverlap`
  (params (OverlappedComponent :type "PrimitiveComponent Object Reference") (OtherActor :type "Actor Object Reference") (OtherComp :type "PrimitiveComponent Object Reference") (OtherBodyIndex :type Integer) (bFromSweep :type Boolean) (SweepResult :type "HitResult Structure (by ref)"))
  (set `self.bScanOn` true))

(event `self.ReceiveBeginPlay`
  (set `self.CannonRange` (`SphereComponent.GetUnscaledSphereRadius` (`self.Sphere`))))

(event `GetClostestPlayer`
  (bind _returnvalue (`SceneComponent.GetSocketLocation` (`self.Barrel`) "Muzzle"))
  (for _array_element (`PrimitiveComponent.GetOverlappingActors` (`self.Sphere`) "/Script/VR_Project.vrPlayer")
    (if (`KismetSystemLibrary.IsValid` (`self.ClosestPlayer`))
      (bind _asvr_player (cast `vrPlayer` _array_element :!pure true))
      (if (< (`KismetMathLibrary.VSize` (- _returnvalue (`self.K2_GetActorLocation` _asvr_player))) (`KismetMathLibrary.VSize` (- _returnvalue (`SceneComponent.K2_GetComponentLocation` (`Character.CapsuleComponent` (`self.ClosestPlayer`))))))
        (set `self.ClosestPlayer` _asvr_player))
      (else
        (set `self.ClosestPlayer` _asvr_player))))
  (if (`KismetSystemLibrary.IsValid` (`self.ClosestPlayer`))
    (`self.CheckClosestestPlayerLOS`)
    (else
      (set `self.bScanOn` false))))

(event `self.HealthStats.DamageTaken`
  (params (HealthStatsComp :type "HealthStats Object Reference") (Health :type "Float (single-precision)") (Damage :type "Float (single-precision)") (DamageType :type "DamageType Object Reference") (InstigatedBy :type "Controller Object Reference") (DamageCauser :type "Actor Object Reference"))
  (bind _returnvalue (`KismetStringLibrary.Conv_DoubleToString` Damage))
  (`KismetSystemLibrary.DrawDebugString` (`SceneComponent.K2_GetComponentLocation` (`self.Barrel`)) _returnvalue null (struct :`R` 1.0 :`G` 0.029373 :`A` 1.0) 1.0)
  (`KismetSystemLibrary.PrintString` _returnvalue)
  (if (== Health 0.0)
    (`self.K2_DestroyActor`)))

(fn `UserConstructionScript`)