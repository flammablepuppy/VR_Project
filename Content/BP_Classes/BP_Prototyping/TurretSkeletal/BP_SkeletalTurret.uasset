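; Prototype turret actor that detects VR players inside its radar sphere and turns toward one, with no actual firing logic yet.
; Tick, throttled by a Delay, scans overlaps and stores a ClosestPlayer, though the distance comparison actually keeps the farthest.
; A debug-drawn muzzle line trace confirms line of sight, then FireOnTarget interpolates separate yaw and pitch meshes toward the target using frame delta time.
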(event `self.ReceiveTick`
  (params (DeltaSeconds :type "Float (single-precision)"))
  (`KismetSystemLibrary.Delay` 0.5)
  (`self.RadarScanForPlayers`))

(event `RadarScanForPlayers`
  (bind _closestplayer (`self.ClosestPlayer`))
  (set `self.ClosestPlayer` null)
  (for _array_element (`PrimitiveComponent.GetOverlappingActors` (`self.RadarSphere`) "/Script/VR_Project.vrPlayer")
    (`/Engine/EditorBlueprintResources/StandardMacros.IsValid` _closestplayer
      (:`Is Valid`
        (bind _asvr_player (cast `vrPlayer` _array_element :!pure true))
        (if (> (`KismetMathLibrary.VSize` (- (`SceneComponent.K2_GetComponentLocation` (`Character.CapsuleComponent` _asvr_player)) (`SceneComponent.K2_GetComponentLocation` (`self.TurretPitchMesh`)))) (`KismetMathLibrary.VSize` (- (`SceneComponent.K2_GetComponentLocation` (`Character.CapsuleComponent` _closestplayer)) (`SceneComponent.K2_GetComponentLocation` (`self.TurretPitchMesh`)))))
          (set `self.ClosestPlayer` _asvr_player)))
      (:`Is Not Valid`
        (set `self.ClosestPlayer` _asvr_player))))
  (if (`KismetSystemLibrary.IsValid` (`self.ClosestPlayer`))
    (`self.CheckInLOS`)))

(event `CheckInLOS`
  (bind _returnvalue (`SceneComponent.GetSocketLocation` (`self.TurretPitchMesh`) "Muzzle"))
  (bind _outhit (`KismetSystemLibrary.LineTraceSingle` :`Start` _returnvalue :`End` (+ _returnvalue (* (- (`SceneComponent.K2_GetComponentLocation` (`Character.CapsuleComponent` (`self.ClosestPlayer`))) _returnvalue) 1.2)) :`TraceChannel` "TraceTypeQuery2" :`bTraceComplex` true :`DrawDebugType` "ForDuration"))
  (bind _returnvalue_2 (`ActorComponent.GetOwner` (`.HitComponent` (`GameplayStatics.BreakHitResult` _outhit))))
  (cast `vrPlayer` _returnvalue_2)
  (`self.FireOnTarget`)
  (`KismetSystemLibrary.PrintString` (`KismetSystemLibrary.GetDisplayName` _returnvalue_2)))

(event `FireOnTarget`
  (bind _turretpitchmesh (`self.TurretPitchMesh`))
  (bind _turretpitchmesh_2 (`self.TurretPitchMesh`))
  (bind (_returnvalue_roll _returnvalue_pitch) (`KismetMathLibrary.BreakRotator` (`KismetMathLibrary.RInterpTo` (`SceneComponent.K2_GetComponentRotation` _turretpitchmesh) (`KismetMathLibrary.FindLookAtRotation` (`SceneComponent.GetSocketLocation` _turretpitchmesh "Muzzle") (`SceneComponent.K2_GetComponentLocation` (`Character.CapsuleComponent` (`self.ClosestPlayer`)))) (`GameplayStatics.GetWorldDeltaSeconds`) (`self.PitchSpeed`))))
  (bind (_returnvalue_roll_2 _returnvalue_pitch_2 _returnvalue_yaw) (`KismetMathLibrary.BreakRotator` (`KismetMathLibrary.RInterpTo` (`SceneComponent.K2_GetComponentRotation` _turretpitchmesh_2) (`KismetMathLibrary.FindLookAtRotation` (`SceneComponent.GetSocketLocation` _turretpitchmesh_2 "Muzzle") (`SceneComponent.K2_GetComponentLocation` (`Character.CapsuleComponent` (`self.ClosestPlayer`)))) (`GameplayStatics.GetWorldDeltaSeconds`) (`self.YawSpeed`))))
  (`SceneComponent.K2_SetWorldRotation` (`self.TurretYawMesh`) (`KismetMathLibrary.MakeRotator` 0.0 0.0 _returnvalue_yaw) false false)
  (`SceneComponent.K2_SetWorldRotation` (`self.TurretPitchMesh`) (`KismetMathLibrary.MakeRotator` 0.0 _returnvalue_pitch) false false))

(fn `UserConstructionScript`)