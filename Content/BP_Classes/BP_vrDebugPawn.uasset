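; BP_vrDebugPawn is a debug pawn for VR that also supports play without a headset.
; On BeginPlay, with an HMD enabled it disables the mouse, sets eye-level tracking origin and raises VrRoot near the capsule top; otherwise it uses controller yaw rotation.
; Highlight and end-highlight events toggle a flag that makes Tick print a "CANPICKUP" message on screen each frame.
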(event `self.BPHighlight`
  (set `self.PickupMessage` true))

(event `self.BPEndHighlight`
  (set `self.PickupMessage` false))

(event `self.ReceiveTick`
  (params (DeltaSeconds :type "Float (single-precision)"))
  (if (`self.PickupMessage`)
    (`KismetSystemLibrary.PrintString` "CANPICKUP" true true (struct :`G` 0.66 :`B` 1.0 :`A` 1.0) 0.0)))

(event `self.ReceiveBeginPlay`
  (if (`HeadMountedDisplayFunctionLibrary.IsHeadMountedDisplayEnabled`)
    (`self.SetMouseEnabled` false)
    (`HeadMountedDisplayFunctionLibrary.SetTrackingOrigin` "Eye")
    (`SceneComponent.K2_SetRelativeLocation` (`self.vrRoot`) (`KismetMathLibrary.MakeVector` 0.0 0.0 (- (`CapsuleComponent.GetScaledCapsuleHalfHeight` (`self.CapsuleComponent`)) 10.0)) false false)
    (else
      (set `self.bUseControllerRotationYaw` true))))

(fn `UserConstructionScript`)