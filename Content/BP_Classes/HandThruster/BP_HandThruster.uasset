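; BP_HandThruster is a hand thruster actor with a pickup mesh and a widget component.
; On BeginPlay it casts the component's user widget to Widget_HandThruster and sets itself as that widget's OwningActor.
; A disconnected debug line trace would visualize ground effect range along the mesh's downward axis over GroundEffectDistance.
; Tick and the construction script are empty, and this graph contains no thrust logic.
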(event `self.ReceiveBeginPlay`
  (bind _aswidget_hand_thruster (cast `/Game/BP_Classes/HandThruster/Widget_HandThruster` (`WidgetComponent.GetUserWidgetObject` (`self.Widget`))))
  (set `/Game/BP_Classes/HandThruster/Widget_HandThruster.OwningActor` self _aswidget_hand_thruster))

(event `self.ReceiveTick`
  (params (DeltaSeconds :type "Float (single-precision)"))
  ;[1 1 1] Ground Effect visualization
)

(fn `UserConstructionScript`)