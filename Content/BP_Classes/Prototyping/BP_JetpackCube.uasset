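; Prototype VR handheld jetpack cube that propels the owning player along the pickup mesh's up vector.
; Trigger pull sets a throttle that drains fuel and scales thrust.
; Grounded players are launched with LaunchCharacter, while falling players get thrust added directly to movement velocity with slight damping.
; The bottom button toggles a throttle lock at a fixed high value, which releases when a trigger update finds fuel empty.
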(event `self.BPTriggerPull`
  (params (Value :type "Float (single-precision)"))
  (bind _fuel (`self.Fuel`))
  (bind _triggerpullvalue (`self.TriggerPullValue`))
  (bind _asvr_player (cast `vrPlayer` (`ActorComponent.GetOwner` (`self.GetOwningMC`)) :!pure true))
  (bind _returnvalue (* (`KismetMathLibrary.GetUpVector` (`SceneComponent.K2_GetComponentRotation` (`self.PickupMesh`))) (* (`self.ThrustPower`) _triggerpullvalue)))
  (bind _returnvalue_2 (`Pawn.GetMovementComponent` _asvr_player))
  (if (> _triggerpullvalue 0.1)
    (if (not (`self.bThrottleLocked`)) :!label _label
      (set `self.TriggerPullValue` Value))
    (if (> _fuel 0.0)
      (set `self.Fuel` (`KismetMathLibrary.FClamp` (- _fuel (* (`GameplayStatics.GetWorldDeltaSeconds`) _triggerpullvalue)) 0.0 (`self.MaxFuel`)))
      (if (`NavMovementComponent.IsFalling` _returnvalue_2)
        (set `MovementComponent.Velocity` (* (+ (`MovementComponent.Velocity` _returnvalue_2) _returnvalue) 0.997) _returnvalue_2)
        (else
          (`Character.LaunchCharacter` _asvr_player _returnvalue false false)))
      (else
        (set `self.bThrottleLocked` false)))
    (elif (> Value 0.1)
      (goto _label))))

(event `self.BPBottomPush`
  (if (`self.bThrottleLocked`)
    (set `self.bThrottleLocked` false)
    (else
      (set `self.bThrottleLocked` true)
      (set `self.TriggerPullValue` 0.85))))

(fn `UserConstructionScript`)