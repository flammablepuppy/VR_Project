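; BP_SigAuto is a Sig pistol weapon that supplies the gun's animation class, sound and muzzle effects.
; The first snap-on spawns a BP_SigHolster on the owning player's utility belt.
; Events play slide, magazine, hammer and shot sounds at the mesh, with slide events also setting the slide bone offset.
; Firing attaches a muzzle flash at the Muzzle socket, then detaches it after a brief delay so it stays in world space.
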(event `self.ReceiveBeginPlay`
  (`SkeletalMeshComponent.K2_SetAnimInstanceClass` (`self.PistolMesh`) "/Game/BP_Classes/SigPistol/SigSauer_SkeletalMesh/SigAnimation.SigAnimation_C")
  (add `self.OnSnappedOn` (delegate `SpawnHolster`)))

(event `SpawnHolster` :!signature `self.OnSnappedOn`
  (params (PickupToEnable :type "vrPickup Object Reference"))
  (if (not (`self.bCreatedHolster`))
    (set `self.bCreatedHolster` true)
    (`vrBelt.SpawnHolster` (`vrPlayer.GetUtilityBelt` (`self.GetOwningPlayer` PickupToEnable)) (10.0 20.0 0.0) "/Game/BP_Classes/vrPawn/Holsters/BP_SigHolster.BP_SigHolster_C" false)))

(event `self.PlaySlideBack`
  ;[1 1 1] TODO: Make Sound Cues with attenuation for these SFX
  (set `self.SlideBonePosition` (-5.0 0.0 0.0))
  (`GameplayStatics.PlaySoundAtLocation` "/Game/BP_Classes/SigPistol/SFX/CartridgeLoad01.CartridgeLoad01" (`SceneComponent.K2_GetComponentLocation` (`self.PistolMesh`)) (struct) 1.0 1.0 0.0 null null null))

(event `self.PlaySlideForward`
  ;[1 1 1] TODO: Make Sound Cues with attenuation for these SFX
  (set `self.SlideBonePosition` (0.0 0.0 0.0))
  (`GameplayStatics.PlaySoundAtLocation` "/Game/BP_Classes/SigPistol/SFX/SlideSnapForward.SlideSnapForward" (`SceneComponent.K2_GetComponentLocation` (`self.PistolMesh`)) (struct) 1.0 1.0 0.0 null null null))

(event `self.BPBottomPush`
  ;[1 1 1] TODO: Make Sound Cues with attenuation for these SFX
  (`GameplayStatics.PlaySoundAtLocation` "/Game/BP_Classes/SigPistol/SFX/EjectMag.EjectMag" (`SceneComponent.K2_GetComponentLocation` (`self.PistolMesh`)) (struct) 1.0 1.0 0.0 null null null))

(event `self.BP_PlayMagLoad`
  ;[1 1 1] TODO: Make Sound Cues with attenuation for these SFX
  (`GameplayStatics.PlaySoundAtLocation` "/Game/BP_Classes/SigPistol/SFX/LoadMag.LoadMag" (`SceneComponent.K2_GetComponentLocation` (`self.PistolMesh`)) (struct) 1.0 1.0 0.0 null null null))

(event `self.BP_PlayHammer`
  ;[1 1 1] TODO: Make Sound Cues with attenuation for these SFX
  (`GameplayStatics.PlaySoundAtLocation` "/Game/BP_Classes/SigPistol/SFX/Hammer.Hammer" (`SceneComponent.K2_GetComponentLocation` (`self.PistolMesh`)) (struct) 1.0 1.0 0.0 null null null))

(event `self.PlayFireFX`
  (bind _pistolmesh (`self.PistolMesh`))
  (bind (_returnvalue_location _returnvalue_rotation) (`KismetMathLibrary.BreakTransform` (`SceneComponent.GetSocketTransform` _pistolmesh "Muzzle" "RTS_World")))
  (`GameplayStatics.SpawnSoundAtLocation` "/Game/BP_Classes/SigPistol/SFX/PistolShot_Cue.PistolShot_Cue" (`SceneComponent.K2_GetComponentLocation` (`self.PistolMesh`)) (struct) 1.0 1.0 0.0 null null)
  (bind _returnvalue (`GameplayStatics.SpawnEmitterAttached` "/Game/BP_Classes/SigPistol/VFX/P_PistolMuzzleFlash.P_PistolMuzzleFlash" _pistolmesh "Muzzle" _returnvalue_location _returnvalue_rotation (0.6 0.6 0.6) "KeepWorldPosition"))
  (`KismetSystemLibrary.Delay` 0.08)
  (`SceneComponent.K2_DetachFromComponent` _returnvalue "KeepWorld" "KeepWorld" "KeepWorld" true))

(fn `UserConstructionScript`)