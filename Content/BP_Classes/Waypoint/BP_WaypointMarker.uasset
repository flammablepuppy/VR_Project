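; Waypoint marker actor that shows a course-colored objective mesh and animates it when collected.
; The construction script creates dynamic materials for both mesh slots and sets the glow color from the course color.
; On BeginPlay, an idle timeline starts driving the mesh's uniform scale.
; The OnCollected event triggers a second timeline that drives the same scale for the collection animation.
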(event `self.ReceiveBeginPlay`
  (add `self.OnCollected` (delegate `AnimateCollection`))
  (bind (_direction _scaleanim) (`Timeline|IdleAnim` :!via `PlayFromStart`)
    (:`Update`
      (`SceneComponent.SetWorldScale3D` (`self.WaypointMesh`) (`KismetMathLibrary.Conv_DoubleToVector` _scaleanim)))))

(event `AnimateCollection`
  (bind (_direction _scale) (`Timeline|CollectionAnimTimeline` :!via `PlayFromStart`)
    (:`Update`
      (`SceneComponent.SetWorldScale3D` (`self.WaypointMesh`) (`KismetMathLibrary.Conv_DoubleToVector` _scale)))))

(fn `UserConstructionScript`
  (bind _waypointmesh (`self.WaypointMesh`))
  (`PrimitiveComponent.CreateDynamicMaterialInstance` _waypointmesh 0 "/Game/BP_Classes/SigPistol/StaticMeshes_Materials/BlackPolymer.BlackPolymer" "None")
  (bind _returnvalue (`PrimitiveComponent.CreateDynamicMaterialInstance` _waypointmesh 1 "/Game/BP_Classes/SigPistol/StaticMeshes_Materials/ObjectiveGlow.ObjectiveGlow" "None"))
  (`MaterialInstanceDynamic.SetVectorParameterValue` _returnvalue "GlowColor" (`KismetMathLibrary.Conv_ColorToLinearColor` (`self.GetCourseColor`))))