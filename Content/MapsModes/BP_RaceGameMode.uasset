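; Race game mode Blueprint with a "floor is lava" rule that damages the VR player on contact with the landscape.
; The TheFloorIsLava event finds VrPlayer actors and binds the first one's OnActorHit to the kill handler.
; On a landscape hit, the handler checks the health stats component and, if the player is alive, plays a pistol-shot sound and applies heavy damage.
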(event `TheFloorIsLava`
  (bind _outactors (`GameplayStatics.GetAllActorsOfClass` "/Script/VR_Project.vrPlayer"))
  (add `Actor.OnActorHit` (`|GetArrayItem` _outactors) (delegate `Floor is Lava Kill`)))

(event `Floor is Lava Kill`
  (params (SelfActor :type "Actor Object Reference") (OtherActor :type "Actor Object Reference") (NormalImpulse :type "Vector Structure") (Hit :type "HitResult Structure (by ref)"))
  (cast `Landscape` OtherActor)
  (bind _asvr_player (cast `vrPlayer` SelfActor))
  (if (not (`HealthStats.GetIsDead` (`vrPlayer.HealthStatsComp` _asvr_player)))
    (`GameplayStatics.PlaySound2D` "/Game/BP_Classes/SigPistol/SFX/PistolShot_Cue.PistolShot_Cue" 1.0 1.0 0.0 null null)
    (`GameplayStatics.ApplyDamage` SelfActor 500.0 null null "/Script/Engine.DamageType")))

(fn `UserConstructionScript`)